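; Player hero for a sprite-based dungeon game, with Enhanced Input movement, sword and bow attacks, and a hearts HUD.
; PaperZD animation overrides set attack and stun flags that gate input, while CheckHit damages overlapping enemies and FireArrow spawns arrows.
; Hits refresh the HUD, grant invincibility, disable the hurtbox and play a stun animation, then start sprite flickering or, on defeat, reload the level after a delay.
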(event Input|EnhancedActionEvents|EnhancedInputActionIA_Move
  (params (ActionValue :type Vector%202D%20Structure) (ElapsedSeconds :type Float%20%28double-precision%29) (TriggeredSeconds :type Float%20%28double-precision%29) (InputAction :type Input%20Action%20Object%20Reference :default "/Game/Input/Action/IA_Move.IA_Move"))
  (bind (_x _y) (Math|Vector2D|BreakVector2D ActionValue))
  (if (CallFunction|PlayerIsAbletoMove)
    (Variables|Default|SetDirectionality ActionValue)
    (Pawn|Input|AddMovementInput "1.000000,0.000000,0.000000" _x false)
    (Pawn|Input|AddMovementInput "0.000000,1.000000,0.000000" _y false)))

(event Input|EnhancedActionEvents|EnhancedInputActionIA_Sword
  (params (ActionValue :type Boolean) (ElapsedSeconds :type Float%20%28double-precision%29) (TriggeredSeconds :type Float%20%28double-precision%29) (InputAction :type Input%20Action%20Object%20Reference :default "/Game/Input/Action/IA_Sword.IA_Sword"))
  (:Started
    (if (CallFunction|PlayerIsAbletoMove)
      (|PlayAnimationOverridewithCallbacks (Variables|/Script/PaperZD.PaperZDAnimationComponent|GetAnimInstance (Variables|Default|GetAnimationComponent)) "/Game/Blueprints/Character/Hero/AnimSequences/Attack.Attack" "DefaultSlot" (Variables|Default|GetSwordAttackPlayRate) 0.0
        (:then
          (Variables|Default|SetIsAttacking true))
        (:OnCompleted
          (Variables|Default|SetIsAttacking false :!label _label))
        (:OnCancelled
          (goto _label))))))

(event Input|EnhancedActionEvents|EnhancedInputActionIA_Bow
  (params (ActionValue :type Boolean) (ElapsedSeconds :type Float%20%28double-precision%29) (TriggeredSeconds :type Float%20%28double-precision%29) (InputAction :type Input%20Action%20Object%20Reference :default "/Game/Input/Action/IA_Bow.IA_Bow"))
  (:Started
    (if (and (CallFunction|PlayerIsAbletoMove) (Variables|Default|GetCanUseBow))
      (|PlayAnimationOverridewithCallbacks (Variables|/Script/PaperZD.PaperZDAnimationComponent|GetAnimInstance (Variables|Default|GetAnimationComponent)) "/Game/Blueprints/Character/Hero/AnimSequences/Bow.Bow" "DefaultSlot" 1.0 0.0
        (:then
          (Variables|Default|SetIsAttacking true))
        (:OnCompleted
          (Variables|Default|SetIsAttacking false :!label _label))
        (:OnCancelled
          (goto _label))))))

(event Input|EnhancedActionEvents|EnhancedInputActionIA_Exit
  (params (ActionValue :type Boolean) (ElapsedSeconds :type Float%20%28double-precision%29) (TriggeredSeconds :type Float%20%28double-precision%29) (InputAction :type Input%20Action%20Object%20Reference :default "/Game/Input/Action/IA_Exit.IA_Exit"))
  (:Started
    (Game|QuitGame 0 "Quit" false)))

(event EventBeginPlay
  (|CallParentFunction)
  (Utilities|FlowControl|Sequence
    (:then_0
      (bind _asplayer_controller (Utilities|Casting|CastToPlayerController (Pawn|GetController)))
      (Input|AddMappingContext (PlayerController|LocalPlayerSubsystems|GetEnhancedInputLocalPlayerSubsystem _asplayer_controller) "/Game/Input/IMC_Dungeon.IMC_Dungeon" 0 "(bIgnoreAllPressedKeysUntilRelease=True,bForceImmediately=False,bNotifyUserSettings=False)"))
    (:then_1
      (bind _returnvalue (UserInterface|CreateWidget "/Game/Widgets/WBP_MainHUD.WBP_MainHUD_C"))
      (bind _output_get (Variables|Default|SetMainHUD _returnvalue))
      (UserInterface|Viewport|AddtoViewport _output_get 0)
      (Default|InitializeHearts (Variables|/Game/Widgets/WBP_MainHUD.WBP_MainHUD_C|GetWBP_HealthBox (Variables|Default|GetMainHUD)) (Variables|/Game/Blueprints/Components/BPC_Health.BPC_Health_C|GetMaxHealth (Variables|Default|GetBPC_Health))))
    (:then_2
      (Transformation|SetWorldLocation (Variables|Default|GetSpringArm) (Transformation|GetActorLocation) false false))))

(event EventHandleHitExtended
  (|CallParentFunction)
  (Default|RefreshCurrentHealth (Variables|/Game/Widgets/WBP_MainHUD.WBP_MainHUD_C|GetWBP_HealthBox (Variables|Default|GetMainHUD)) (Variables|/Game/Blueprints/Components/BPC_Health.BPC_Health_C|GetCurrentHealth (Variables|Default|GetBPC_Health)))
  (Default|SetInvincibility (Variables|Default|GetBPC_Health))
  (Collision|SetCollisionEnabled (Variables|Default|GetHurtBox) "NoCollision")
  (|PlayAnimationOverridewithCallbacks (Variables|/Script/PaperZD.PaperZDAnimationComponent|GetAnimInstance (Variables|Default|GetAnimationComponent)) (Variables|Default|GetGetHitAnim) "DefaultSlot" 1.0 0.0
    (:then
      (Variables|Default|SetIsStunned true))
    (:OnCompleted
      (Variables|Default|SetIsStunned false :!label _label)
      (CallFunction|HitStop)
      (if (Variables|/Game/Blueprints/Components/BPC_Health.BPC_Health_C|GetIsDefeated (Variables|Default|GetBPC_Health))
        (Class|PaperZDAnimInstance|JumptoNode (Variables|/Script/PaperZD.PaperZDAnimationComponent|GetAnimInstance (Variables|Default|GetAnimationComponent)) "DefeatJump" "None")
        (Default|CallPlayerDefeated)
        (Utilities|FlowControl|Delay 2.0)
        (bind _returnvalue (Game|GetCurrentLevelName true))
        (Game|OpenLevel(byName) (Utilities|String|StringToName _returnvalue))
        (else
          (bind _returnvalue_2 (Utilities|Time|SetTimerbyEvent (EventDispatchers|CreateEvent :!event SetSpriteVisibility) (Variables|Default|GetSpriteFlickeringInterval) true))
          (Variables|Default|SetFlickerHandle _returnvalue_2))))
    (:OnCancelled
      (goto _label))))

(fn ConstructionScript
  (|CallParentFunction))

(fn PlayerIsAbletoMove
  (return (Math|Boolean|ANDBoolean (not (Variables|Default|GetIsStunned)) (not (Variables|/Game/Blueprints/Components/BPC_Health.BPC_Health_C|GetIsDefeated (Variables|Default|GetBPC_Health))) (not (Variables|Default|GetIsAttacking)))))

(fn CheckHit
  (bind _arrayelement (Utilities|Array|ReverseforEachLoop (Collision|GetOverlappingActors (Variables|Default|GetHitbox) "/Game/Blueprints/Character/BP_Enemy_BASE.BP_Enemy_BASE_C" :!class /Script/Engine.PrimitiveComponent))
    (:LoopBody
      (Game|Damage|ApplyDamage _arrayelement (Variables|Default|GetSwordDamage) 0 self))))

(fn FireArrow
  (bind _arrowpos (Variables|Default|GetArrowPos))
  (bind _returnvalue (Transformation|GetWorldTransform _arrowpos))
  (Game|SpawnActorfromClass "/Game/Blueprints/Projectiles/BP_Hero_Arrow.BP_Hero_Arrow_C" (Math|Transform|MakeTransform (.location _returnvalue) (.rotation _returnvalue) "1.000000,1.000000,1.000000") "Undefined" "MultiplyWithRoot" self 0))

(fn GetHeal
  (params (IncreaseAmount :type Float%20%28double-precision%29))
  (Default|IncreaseHealth (Variables|Default|GetBPC_Health) IncreaseAmount)
  (Default|RefreshCurrentHealth (Variables|/Game/Widgets/WBP_MainHUD.WBP_MainHUD_C|GetWBP_HealthBox (Variables|Default|GetMainHUD)) (Variables|/Game/Blueprints/Components/BPC_Health.BPC_Health_C|GetCurrentHealth (Variables|Default|GetBPC_Health))))
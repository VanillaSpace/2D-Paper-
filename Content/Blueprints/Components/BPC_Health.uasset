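; Health component that tracks an actor's current health, defeat state and temporary invincibility.
; Health starts at the maximum on BeginPlay, and decrease and increase functions clamp it between zero and max, with the decrease also setting the defeated flag.
; A retriggerable delay times the invincibility window and fires an expired dispatcher when it ends.
; CanBeDamage reports false while defeated or invincible, but damage reduction itself does not check it.
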(event Custom|SetInvincibility
  (Variables|Default|SetIsInvincible true)
  (Utilities|FlowControl|RetriggerableDelay (Variables|Default|GetIncincibilityDuration))
  (Variables|Default|SetIsInvincible false)
  (Default|CallInvincibilityExpired))

(event EventBeginPlay
  (Variables|Default|SetCurrentHealth (Variables|Default|GetMaxHealth)))

(fn DreacreaseHealth
  (params (IncomingDamage :type Float%20%28double-precision%29))
  (Variables|Default|SetCurrentHealth (Math|Float|Max(Float) (- (Variables|Default|GetCurrentHealth) IncomingDamage) 0.0))
  (Variables|Default|SetIsDefeated (<= (Variables|Default|GetCurrentHealth) 0.0)))

(fn CanbeDamage
  (return (and (not (Variables|Default|GetIsDefeated)) (not (Variables|Default|GetIsInvincible)))))

(fn IncreaseHealth
  (params (IncreaseAmount :type Float%20%28double-precision%29))
  (Variables|Default|SetCurrentHealth (Math|Float|Min(Float) (+ (Variables|Default|GetCurrentHealth) IncreaseAmount) (Variables|Default|GetMaxHealth))))